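; BossEnemy is an enemy Blueprint for a boss that shows a health bar on player HUDs.
; On BeginPlay it creates a BossHealth widget for each BaseCharacterPawn, adds it to that pawn's HUD and links it back to the boss.
; AnyDamage lowers clamped Health and plays a hitmarker on the instigating player controller.
; The zero-health check leads to no logic, so death is not handled here.
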(event `self.ReceiveBeginPlay`
  (bind _outactors (`GameplayStatics.GetAllActorsOfClass` "/Game/GameFiles/Blueprints/Character/BaseCharacterPawn.BaseCharacterPawn_C"))
  (for _array_element _outactors
    (bind _asbase_character_pawn (cast `/Game/GameFiles/Blueprints/Character/BaseCharacterPawn` _array_element))
    (bind _returnvalue (`|CreateWidget` "/Game/GameFiles/Blueprints/HUD/BossHealth.BossHealth_C"))
    (`/Game/GameFiles/Blueprints/HUD/GameHUD.AddBossbar` (`/Game/GameFiles/Blueprints/Character/BaseCharacterPawn.GameHUDRef` _asbase_character_pawn) _returnvalue)
    (set `/Game/GameFiles/Blueprints/HUD/BossHealth.OwningBoss` self _returnvalue)))

(event `self.ReceiveAnyDamage`
  (params (Damage :type "Float (single-precision)") (DamageType :type "DamageType Object Reference") (InstigatedBy :type "Controller Object Reference") (DamageCauser :type "Actor Object Reference"))
  (set `self.Health` (`KismetMathLibrary.FClamp` (- (`self.Health`) Damage) 0.0 (`self.MaxHealth`)))
  (bind _asbp_player_controller (cast `/Game/GameFiles/Blueprints/Basics/BP_PlayerController` InstigatedBy))
  (`/Game/GameFiles/Blueprints/Basics/BP_PlayerController.PlayHitmarker` _asbp_player_controller)
  (if (<= (`self.Health`) 0.0)
    _))

(fn `UserConstructionScript`)