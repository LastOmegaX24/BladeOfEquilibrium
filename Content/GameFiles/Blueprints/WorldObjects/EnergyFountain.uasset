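; EnergyFountain is a world object that periodically emits EnergyParticle actors from an Arrow component.
; Tick feeds a five-second Delay, which ignores retriggers while pending and so acts as a repeating spawn timer.
; Each particle spawns at the arrow's location, with random Spread offsets added to its roll, pitch and yaw.
; Spawning adjusts for collisions where possible and is skipped if still colliding.
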(event `self.ReceiveTick`
  (params (DeltaSeconds :type "Float (single-precision)"))
  (bind _spread (`self.Spread`))
  (bind _returnvalue (`SceneComponent.K2_GetComponentToWorld` (`self.Arrow`)))
  (bind _returnvalue_2 (* _spread -1.0))
  (`KismetSystemLibrary.Delay` 5.0)
  (`|SpawnActorFromClass` "/Game/GameFiles/Blueprints/Ability/EnergySystem/EnergyParticle.EnergyParticle_C" (`KismetMathLibrary.MakeTransform` (.location _returnvalue) (`KismetMathLibrary.MakeRotator` (+ (`KismetMathLibrary.RandomFloatInRange` _returnvalue_2 _spread) (.roll (.rotation _returnvalue))) (+ (`KismetMathLibrary.RandomFloatInRange` _returnvalue_2 _spread) (.pitch (.rotation _returnvalue))) (+ (`KismetMathLibrary.RandomFloatInRange` _returnvalue_2 _spread) (.yaw (.rotation _returnvalue))))) "AdjustIfPossibleButDontSpawnIfColliding" "MultiplyWithRoot" null null))

(fn `UserConstructionScript`)