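; A destroyable world object that releases energy particles when damage depletes its health.
; Any damage lowers its clamped health and plays a hitmarker when the instigator is a BP_PlayerController.
; At zero health it spawns several EnergyParticle actors from its Arrow component, each with a random rotational spread, then plays an explosion effect and destroys itself.
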(event `self.ReceiveAnyDamage`
  (params (Damage :type "Float (single-precision)") (DamageType :type "DamageType Object Reference") (InstigatedBy :type "Controller Object Reference") (DamageCauser :type "Actor Object Reference"))
  (bind _spread (`self.Spread`))
  (bind _returnvalue (`SceneComponent.K2_GetComponentToWorld` (`self.Arrow`)))
  (bind _returnvalue_2 (* _spread -1.0))
  (set `self.Health` (`KismetMathLibrary.FClamp` (- (`self.Health`) Damage) 0.0 (`self.MaxHealth`)))
  (bind _asbp_player_controller (cast `/Game/GameFiles/Blueprints/Basics/BP_PlayerController` InstigatedBy)
    (:`then`
      (`/Game/GameFiles/Blueprints/Basics/BP_PlayerController.PlayHitmarker` _asbp_player_controller))
    (:`CastFailed`
      _))
  (if (<= (`self.Health`) 0.0)
    (for _ (range 6)
      (`|SpawnActorFromClass` "/Game/GameFiles/Blueprints/Ability/EnergySystem/EnergyParticle.EnergyParticle_C" (`KismetMathLibrary.MakeTransform` (.location _returnvalue) (`KismetMathLibrary.MakeRotator` (+ (`KismetMathLibrary.RandomFloatInRange` _returnvalue_2 _spread) (.roll (.rotation _returnvalue))) (+ (`KismetMathLibrary.RandomFloatInRange` _returnvalue_2 _spread) (.pitch (.rotation _returnvalue))) (+ (`KismetMathLibrary.RandomFloatInRange` _returnvalue_2 _spread) (.yaw (.rotation _returnvalue))))) "AlwaysSpawn" "MultiplyWithRoot" null null))
    (`NiagaraFunctionLibrary.SpawnSystemAtLocation` "/Niagara/DefaultAssets/Templates/Systems/SimpleExplosion.SimpleExplosion" (`self.K2_GetActorLocation`))
    (`self.K2_DestroyActor`)))

(fn `UserConstructionScript`)