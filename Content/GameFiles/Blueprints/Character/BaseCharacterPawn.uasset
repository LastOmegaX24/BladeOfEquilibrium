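; Base player character for a third-person shooter, with health, a gun, a combat camera mode and three ability slots.
; BeginPlay adds input mapping, links the overhead widget and game HUD, then calls a server RPC to spawn an assault rifle attached to an arrow component.
; Tick traces from the combat camera to update the look-at point.
; Input toggles cameras, fires the gun and queues tagged abilities on the AbilitySystemComponent.
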(event `self.ReceiveTick`
  (params (DeltaSeconds :type "Float (single-precision)"))
  (bind _thirdpersoncombatcam (`self.ThirdPersonCombatCam`))
  (bind _returnvalue (`SceneComponent.K2_GetComponentLocation` _thirdpersoncombatcam))
  (bind (_outhit _returnvalue_2) (`KismetSystemLibrary.LineTraceSingleForObjects` :`Start` _returnvalue :`End` (+ _returnvalue (* (`SceneComponent.GetForwardVector` _thirdpersoncombatcam) (`self.SeeRange`))) :`ObjectTypes` (`|MakeArray` "ObjectTypeQuery1" "ObjectTypeQuery3" :!type "EObjectTypeQuery Enum") :`DrawDebugType` "ForOneFrame"))
  (if _returnvalue_2
    (bind (_bblockinghit _binitialoverlap _time _distance _location _impactpoint _normal _impactnormal _physmat _hitactor _hitcomponent _hitbonename _bonename _hititem _elementindex _faceindex _tracestart _traceend) (`GameplayStatics.BreakHitResult` _outhit))
    (set `self.LookAtPoint` _impactpoint)
    (else
      (set `self.LookAtPoint` _traceend))))

(event `self.ReceiveBeginPlay`
  (bind _returnvalue (pcsubsystem `EnhancedInputLocalPlayerSubsystem` (`GameplayStatics.GetPlayerController` 0)))
  (`/Engine/EditorBlueprintResources/StandardMacros.IsValid` _returnvalue
    (:`Is Valid`
      (`EnhancedInputSubsystemInterface.AddMappingContext` _returnvalue "/Game/GameFiles/Input/Keyboard_n_Mouse.Keyboard_n_Mouse" 0 (struct))
      (bind _ascharacter_hud (cast `/Game/GameFiles/Blueprints/HUD/CharacterHUD` (`WidgetComponent.GetWidget` (`self.Widget`))))
      (bind _output_get (set `self.As Character HUD` _ascharacter_hud))
      (set `/Game/GameFiles/Blueprints/HUD/CharacterHUD.OwningCharacter` self _output_get)
      (bind _returnvalue_2 (`|CreateWidget` "/Game/GameFiles/Blueprints/HUD/GameHUD.GameHUD_C" (`GameplayStatics.GetPlayerController` 0)))
      (bind _output_get_2 (set `self.GameHudRef` _returnvalue_2))
      (set `/Game/GameFiles/Blueprints/HUD/GameHUD.OwningCharacter` self _output_get_2)
      (`UserWidget.AddToViewport` _output_get_2 0)
      (bind _asbp_player_controller (cast `/Game/GameFiles/Blueprints/Basics/BP_PlayerController` (`GameplayStatics.GetPlayerController` 0)))
      (bind _output_get_3 (set `self.As BP Player Controller` _asbp_player_controller))
      (set `/Game/GameFiles/Blueprints/Basics/BP_PlayerController.GameHudRef` (`self.GameHUDRef`) _output_get_3)
      (`self.RPC_Server_SpawnGun`))))

(event `RPC_Server_SpawnGun`
  (bind _returnvalue (`|SpawnActorFromClass` "/Game/GameFiles/Blueprints/Weapons/Gun/Guns/AssaultRifle.AssaultRifle_C" (`SceneComponent.K2_GetComponentToWorld` (`self.Arrow1`)) "AlwaysSpawn" "MultiplyWithRoot" self self))
  (bind _output_get (set `self.GunRef` _returnvalue))
  (`self.K2_AttachToComponent` _output_get (`self.Arrow1`) "None" "SnapToTarget" "SnapToTarget" "KeepRelative" true))

(event `self.ReceiveAnyDamage`
  (params (Damage :type "Float (single-precision)") (DamageType :type "DamageType Object Reference") (InstigatedBy :type "Controller Object Reference") (DamageCauser :type "Actor Object Reference"))
  (set `self.Health` (- (`self.Health`) Damage)))

(event `EnhancedInput|/Game/GameFiles/Input/Inputs/SwapCombatMode`
  (params (ActionValue :type Boolean) (ElapsedSeconds :type "Float (double-precision)") (TriggeredSeconds :type "Float (double-precision)") (InputAction :type "InputAction Object Reference" :default "/Game/GameFiles/Input/Inputs/SwapCombatMode.SwapCombatMode"))
  (:`Started`
    (`/Engine/EditorBlueprintResources/StandardMacros.FlipFlop`
      (:`A`
        (set `self.IsCombatMode` true)
        (`ActorComponent.SetActive` (`self.ThirdPersonCombatCam`) true false)
        (`ActorComponent.SetActive` (`self.ThirdPersonCam`) false false))
      (:`B`
        (set `self.IsCombatMode` false)
        (`ActorComponent.SetActive` (`self.ThirdPersonCam`) true false)
        (`ActorComponent.SetActive` (`self.ThirdPersonCombatCam`) false false)))))

(event `EnhancedInput|/Game/GameFiles/Input/Inputs/AbilityPrim`
  (params (ActionValue :type Boolean) (ElapsedSeconds :type "Float (double-precision)") (TriggeredSeconds :type "Float (double-precision)") (InputAction :type "InputAction Object Reference" :default "/Game/GameFiles/Input/Inputs/AbilityPrim.AbilityPrim"))
  (:`Started`
    (`GMC_AbilitySystemComponent.QueueAbility` (`self.AbilitySystemComponent`) (`self.AbPrimary`) InputAction)))

(event `EnhancedInput|/Game/GameFiles/Input/Inputs/AbilitySec`
  (params (ActionValue :type Boolean) (ElapsedSeconds :type "Float (double-precision)") (TriggeredSeconds :type "Float (double-precision)") (InputAction :type "InputAction Object Reference" :default "/Game/GameFiles/Input/Inputs/AbilitySec.AbilitySec"))
  (:`Started`
    (`GMC_AbilitySystemComponent.QueueAbility` (`self.AbilitySystemComponent`) (`self.AbSecondary`) InputAction)))

(event `EnhancedInput|/Game/GameFiles/Input/Inputs/Attack`
  (params (ActionValue :type Boolean) (ElapsedSeconds :type "Float (double-precision)") (TriggeredSeconds :type "Float (double-precision)") (InputAction :type "InputAction Object Reference" :default "/Game/GameFiles/Input/Inputs/Attack.Attack"))
  (bind _gunref (`self.GunRef`))
  (:`Triggered`
    (`/Engine/EditorBlueprintResources/StandardMacros.IsValid` _gunref
      (:`Is Valid`
        (`/Game/GameFiles/Blueprints/Weapons/WeaponBaseClass.Attack` _gunref))))
  (:`Canceled`
    (`/Engine/EditorBlueprintResources/StandardMacros.IsValid` _gunref :!label _label
      (:`Is Valid`
        (`/Game/GameFiles/Blueprints/Weapons/WeaponBaseClass.StopAttack` _gunref))))
  (:`Completed`
    (goto _label)))

(event `EnhancedInput|/Game/GameFiles/Input/Inputs/AbilityUlt`
  (params (ActionValue :type Boolean) (ElapsedSeconds :type "Float (double-precision)") (TriggeredSeconds :type "Float (double-precision)") (InputAction :type "InputAction Object Reference" :default "/Game/GameFiles/Input/Inputs/AbilityUlt.AbilityUlt"))
  (:`Started`
    (`GMC_AbilitySystemComponent.QueueAbility` (`self.AbilitySystemComponent`) (`self.AbUltimate`) InputAction)))

(fn `UserConstructionScript`)