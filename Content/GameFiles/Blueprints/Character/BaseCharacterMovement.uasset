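; GMC-based player character movement component that handles Enhanced Input, camera look and turning, with a toggleable combat mode.
; Binds input and rotation state for replication and forwards prediction, simulation and ancillary ticks to the GMC ability component, whose SprintSpeed attribute sets max speed.
; Combat look yaws the pawn; otherwise the spring arm orbits and the pawn lerps toward camera-relative input.
; Alt plus move in combat queues a Dash ability.
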(event `self.ReceiveBeginPlay`
  (bind _returnvalue (pcsubsystem `EnhancedInputLocalPlayerSubsystem` (`GameplayStatics.GetPlayerController` 0)))
  (`/Engine/EditorBlueprintResources/StandardMacros.IsValid` _returnvalue
    (:`Is Valid`
      (`EnhancedInputSubsystemInterface.AddMappingContext` _returnvalue "/Game/GameFiles/Input/Keyboard_n_Mouse.Keyboard_n_Mouse" 0 (struct))
      (bind _asbase_character_pawn (cast `/Game/GameFiles/Blueprints/Character/BaseCharacterPawn` (`self.GetGMCPawnOwner`)))
      (set `self.Base Character Pawn Ref` _asbase_character_pawn))))

(event `EnhancedInput|/Game/GameFiles/Input/Inputs/MoveXY`
  (params (ActionValue :type "Vector2D Structure") (ElapsedSeconds :type "Float (double-precision)") (TriggeredSeconds :type "Float (double-precision)") (InputAction :type "InputAction Object Reference" :default "/Game/GameFiles/Input/Inputs/MoveXY.MoveXY"))
  (:`Triggered`
    (set `self.MoveXY` ActionValue))
  (:`Started`
    (set `self.IsTurning` true))
  (:`Canceled`
    (set `self.IsTurning` false :!label _label))
  (:`Completed`
    (goto _label)))

(event `EnhancedInput|/Game/GameFiles/Input/Inputs/CameraLook`
  (params (ActionValue :type "Vector2D Structure") (ElapsedSeconds :type "Float (double-precision)") (TriggeredSeconds :type "Float (double-precision)") (InputAction :type "InputAction Object Reference" :default "/Game/GameFiles/Input/Inputs/CameraLook.CameraLook"))
  (bind _returnvalue (`self.GetPhysDeltaTime`))
  (bind _base_character_pawn_ref (`self.Base Character Pawn Ref`))
  (bind _mouse_sensitivity (`self.Mouse Sensitivity`))
  (bind _returnvalue_2 (* _mouse_sensitivity ActionValue_Y _returnvalue))
  (bind _returnvalue_3 (* _mouse_sensitivity ActionValue_X _returnvalue))
  (:`Triggered`
    (`/Engine/EditorBlueprintResources/StandardMacros.IsValid` _base_character_pawn_ref
      (:`Is Valid`
        (if (`self.IsCombatMode`)
          (`Actor.K2_AddActorLocalRotation` _base_character_pawn_ref (`KismetMathLibrary.MakeRotator` 0.0 0.0 _returnvalue_3) false false)
          (`SceneComponent.K2_AddLocalRotation` (`/Game/GameFiles/Blueprints/Character/BaseCharacterPawn.CombatCameraRoot` _base_character_pawn_ref) (`KismetMathLibrary.MakeRotator` 0.0 _returnvalue_2) false false)
          (else
            (`SceneComponent.K2_AddRelativeRotation` (`/Game/GameFiles/Blueprints/Character/BaseCharacterPawn.CameraSpringArm` _base_character_pawn_ref) (`KismetMathLibrary.MakeRotator` 0.0 _returnvalue_2 _returnvalue_3) false false)))))))

(event `self.BindReplicationData`
  (`parent.BindReplicationData`)
  (bind _output_get (set `self.AbilityComponent` (`Actor.GetComponentByClass` (`self.GetPawnOwner`) "/Script/GMCAbilitySystem.GMC_AbilitySystemComponent")))
  (set `GMC_AbilitySystemComponent.GMCMovementComponent` self _output_get)
  (`GMC_AbilitySystemComponent.BindReplicationData` (`self.AbilityComponent`))
  (`self.BindBool` (`self.IsCombatMode`) "ClientAuth_Input" "AlwaysCombine" "Periodic_Output" "NearestNeighbour")
  (`self.BindDoublePrecisionFloat` (`self.Character Yaw`) "ClientAuth_Input" "CombineIfUnchanged" "Periodic_Output" "NearestNeighbour")
  (`self.BindCompressedVector2D` (`self.MoveXY`) "ClientAuth_Input" "CombineIfUnchanged" "Periodic_Output" "NearestNeighbour")
  (`self.BindBool` (`self.IsAltMove`) "ClientAuth_Input" "CombineIfUnchanged" "Periodic_Output" "NearestNeighbour")
  (`self.BindCompressedRotator` (`self.Rotator`) "ClientAuth_Input" "Default" "Periodic_InputOutput" "NearestNeighbour")
  (`self.BindActorReference` (`self.Base Character Pawn Ref`) "ClientAuth_Input" "AlwaysCombine" "Periodic_Output" "NearestNeighbour")
  (`self.BindBool` (`self.IsTurning`) "ClientAuth_Input" "CombineIfUnchanged" "Periodic_Output" "NearestNeighbour"))

(event `self.PreLocalMoveExecution`
  (params (LocalMove :type "GMC_Move Structure (by ref)"))
  (`parent.PreLocalMoveExecution` LocalMove)
  (`GMC_AbilitySystemComponent.PreLocalMoveExecution` (`self.AbilityComponent`)))

(event `EnhancedInput|/Game/GameFiles/Input/Inputs/AltMoveKey`
  (params (ActionValue :type Boolean) (ElapsedSeconds :type "Float (double-precision)") (TriggeredSeconds :type "Float (double-precision)") (InputAction :type "InputAction Object Reference" :default "/Game/GameFiles/Input/Inputs/AltMoveKey.AltMoveKey"))
  (:`Triggered`
    (set `self.IsAltMove` true))
  (:`Canceled`
    (set `self.IsAltMove` false :!label _label_2))
  (:`Completed`
    (goto _label_2)))

(event `EnhancedInput|/Game/GameFiles/Input/Inputs/MoveXY`
  (params (ActionValue :type "Vector2D Structure") (ElapsedSeconds :type "Float (double-precision)") (TriggeredSeconds :type "Float (double-precision)") (InputAction :type "InputAction Object Reference" :default "/Game/GameFiles/Input/Inputs/MoveXY.MoveXY"))
  (:`Started`
    (if (and (`self.IsAltMove`) (`self.IsCombatMode`))
      (`GMC_AbilitySystemComponent.QueueAbility` (`GMAS_Pawn.AbilitySystemComponent` (`self.Base Character Pawn Ref`)) (struct :`TagName` "Ability.Dash") null))))

(event `self.GenAncillaryTick`
  (params (DeltaTime :type "Float (single-precision)") (bLocalMove :type Boolean) (bCombinedClientMove :type Boolean))
  (`parent.GenAncillaryTick` DeltaTime bLocalMove bCombinedClientMove)
  (`GMC_AbilitySystemComponent.GenAncillaryTick` (`self.AbilityComponent`) DeltaTime bCombinedClientMove))

(event `self.GenSimulationTick`
  (params (DeltaTime :type "Float (single-precision)"))
  (`parent.GenSimulationTick` DeltaTime)
  (`GMC_AbilitySystemComponent.GenSimulationTick` (`self.AbilityComponent`) DeltaTime))

(event `EnhancedInput|/Game/GameFiles/Input/Inputs/SwapCombatMode`
  (params (ActionValue :type Boolean) (ElapsedSeconds :type "Float (double-precision)") (TriggeredSeconds :type "Float (double-precision)") (InputAction :type "InputAction Object Reference" :default "/Game/GameFiles/Input/Inputs/SwapCombatMode.SwapCombatMode"))
  (:`Started`
    (`/Engine/EditorBlueprintResources/StandardMacros.FlipFlop`
      (:`A`
        (set `self.IsCombatMode` true))
      (:`B`
        (set `self.IsCombatMode` false)))))

(event `self.GenPredictionTick`
  (params (DeltaTime :type "Float (single-precision)"))
  (`parent.GenPredictionTick` DeltaTime)
  (`GMC_AbilitySystemComponent.GenPredictionTick` (`self.AbilityComponent`) DeltaTime)
  (`self.NonCombatTurn`))

(event `self.MovementUpdate`
  (params (DeltaSeconds :type "Float (single-precision)"))
  (`parent.MovementUpdate` DeltaSeconds)
  (set `self.MaxDesiredSpeed` (`GMC_AbilitySystemComponent.GetAttributeValueByTag` (`self.AbilityComponent`) (struct :`TagName` "Attribute.SprintSpeed"))))

(event `Key|Five`
  (params (Key :type "Key Structure"))
  (:`Pressed`
    (`|K2Node_PlayMontage` null "/Game/GameFiles/Animations/Combat/NewAnimMontage.NewAnimMontage")))

(fn `NonCombatTurn`
  (bind (_movexy_x _movexy_y) (`KismetMathLibrary.BreakVector2D` (`self.MoveXY`)))
  (bind _base_character_pawn_ref (`self.Base Character Pawn Ref`))
  (bind _returnvalue (`SpringArmComponent.GetTargetRotation` (`/Game/GameFiles/Blueprints/Character/BaseCharacterPawn.CameraSpringArm` _base_character_pawn_ref)))
  (if (`self.IsTurning`)
    (if (`self.IsCombatMode`)
      (`Controller.SetControlRotation` (`GameplayStatics.GetPlayerController` 0) (`Actor.K2_GetActorRotation` (`self.GetGMCPawnOwner`)))
      (else
        (`/Engine/EditorBlueprintResources/StandardMacros.IsValid` _base_character_pawn_ref
          (:`Is Valid`
            (bind _output_get (set `self.Rotator` (`KismetMathLibrary.RLerp` (`self.Rotator`) (`KismetMathLibrary.ComposeRotators` (`KismetMathLibrary.Conv_VectorToRotator` (`KismetMathLibrary.MakeVector` _movexy_x _movexy_y)) _returnvalue) 0.1 true)))
            (`Actor.K2_SetActorRotation` _base_character_pawn_ref (`KismetMathLibrary.MakeRotator` 0.0 0.0 (.yaw _output_get)) false)
            (`Controller.SetControlRotation` (`GameplayStatics.GetPlayerController` 0) _returnvalue)))))))